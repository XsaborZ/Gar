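; Game instance Blueprint that handles level loading and quitting the game.
; LoadLevelSafe opens a level by name from the GameLevels array after validating the index, and prints a placeholder debug string when the index is invalid.
; LoadFirstLevel passes a hardcoded index of 1 to it, leaving the FirstLevelIndex variable unused.
; QuitTheGame exits the application.
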(event `LoadFirstLevel`
  (`self.LoadLevelSafe` 1))

(event `QuitTheGame`
  (`KismetSystemLibrary.QuitGame` null "Quit"))

(fn `LoadLevelSafe`
  (params (LevelIndex :type Integer))
  (if (`KismetArrayLibrary.Array_IsValidIndex` (`self.GameLevels`) LevelIndex)
    (`GameplayStatics.OpenLevel` (`|GetArrayItem` (`self.GameLevels`) LevelIndex))
    (else
      (`KismetSystemLibrary.PrintString` "Hello"))))