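; BP_Projectile is a damaging projectile actor with configurable damage, collider scale and lifetime.
; Construction scales the sphere collider and binds its begin-overlap event; BeginPlay starts a one-shot DestroyTime timer and caches the owner as instigating controller.
; HandleOverlap applies damage to the other actor, credited to that controller, then destroys the projectile.
; A failed owner-to-Controller cast only prints a placeholder debug string.
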(event `self.ReceiveBeginPlay`
  (`parent.ReceiveBeginPlay`)
  (`KismetSystemLibrary.K2_SetTimerDelegate` (`|CreateDelegate` :!event `K2_DestroyActor`) (`self.Destroy time`))
  (bind _ascontroller (cast `Controller` (`self.GetOwner`))
    (:`then`
      (set `self.OwnerController` _ascontroller))
    (:`CastFailed`
      (`KismetSystemLibrary.PrintString` "Hello"))))

(fn `HandleOverlap`
  (params (OverlappedComponent :type "PrimitiveComponent Object Reference") (OtherActor :type "Actor Object Reference") (OtherComp :type "PrimitiveComponent Object Reference") (OtherBodyIndex :type Integer) (bFromSweep :type Boolean) (SweepResult :type "HitResult Structure (by ref)"))
  (`GameplayStatics.ApplyDamage` OtherActor (`self.Damage`) (`self.OwnerController`) self)
  (`self.K2_DestroyActor`)
  (return))

(fn `UserConstructionScript`
  (add `PrimitiveComponent.OnComponentBeginOverlap` (`self.sphere collider`) (`|CreateDelegate` :!event `HandleOverlap`))
  (`SceneComponent.SetWorldScale3D` (`self.sphere collider`) (`self.Scale`)))