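; Base rifle actor that fires projectiles for its parent Pawn, and destroys itself on BeginPlay if it has none.
; Attack spawns a projectile at the weapon socket along the Pawn's aim, sets ActionHappening, starts a ResetTime timer and calls OnRifleAttack.
; CanShoot reports when no action is happening, but Attack runs unconditionally and nothing here clears the flag.
; Ammo is not consumed: UseAmmo just sets CurrentAmmo to MaxAmmo.
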(event `CustomEvent`
  (`parent.ReceiveBeginPlay`)
  (bind _aspawn (cast `Pawn` (`self.GetParentActor`))
    (:`then`
      (set `self.ParentPawn` _aspawn))
    (:`CastFailed`
      (`KismetSystemLibrary.PrintString` "Need a pawn to won this rifle")
      (`self.K2_DestroyActor`))))

(event `self.ReceiveBeginPlay`
  (`parent.ReceiveBeginPlay`)
  (bind _aspawn (cast `Pawn` (`self.GetParentActor`))
    (:`then`
      (set `self.ParentPawn` _aspawn))
    (:`CastFailed`
      (`KismetSystemLibrary.PrintString` "owner failed to spawn")
      (`self.K2_DestroyActor`))))

(event `UseAmmo`
  (set `self.CurrentAmmo` (`self.MaxAmmo`)))

(fn `Attack`
  (bind _parentpawn (`self.ParentPawn`))
  (if true
    (`|SpawnActorFromClass` (`self.ProjectileClass`) (`KismetMathLibrary.MakeTransform` (`SceneComponent.GetSocketLocation` (`self.SkeletalMesh`) (`self.WeaponSocketName`)) (`Pawn.GetBaseAimRotation` _parentpawn)) "Undefined" "MultiplyWithRoot" (`Pawn.GetController` _parentpawn) _parentpawn)
    (set `self.Action Happening` true)
    (`KismetSystemLibrary.K2_SetTimerDelegate` :`Time` (`self.reset time`))
    (`self.OnRifleAttack`)))

(fn `CanShoot`
  (returns (CanShoot :type Boolean))
  (return (not (`self.Action Happening`))))

(fn `UserConstructionScript`)