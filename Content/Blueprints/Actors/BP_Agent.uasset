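; BP_Agent is an AI-controlled enemy agent with a weapon and a color tint applied to its mesh materials in the construction script.
; EnemyAttack and EnemyReload pass straight through to the weapon object, which also reloads on BeginPlay.
; BeginPlay binds to the weapon's ammo-changed event, and UpdateBlackBoardAmmo writes the current ammo count to the AI controller's blackboard.
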(event `/Game/Blueprints/utility/BI_EnemyInterface.EnemyReload`
  (`/Game/Blueprints/Actors/BP_BaseRifle.ReloadAmmo` (`self.WeaponObject`)))

(event `/Game/Blueprints/utility/BI_EnemyInterface.Enemy Attack`
  (`/Game/Blueprints/Actors/BP_BaseRifle.Attack` (`self.WeaponObject`)))

(event `self.ReceiveBeginPlay`
  (bind _weaponobject (`self.WeaponObject`))
  (add `/Game/Blueprints/Actors/BP_BaseRifle.OnAmmoChanged` _weaponobject (`|CreateDelegate` :!event `UpdateBlackBoardAmmo`))
  (`/Game/Blueprints/Actors/BP_BaseRifle.ReloadAmmo` _weaponobject))

(fn `UpdateBlackBoardAmmo`
  (params (Current :type "Float (double-precision)") (Max :type "Float (double-precision)"))
  (`BlackboardComponent.SetValueAsFloat` (`AIBlueprintHelperLibrary.GetBlackboard` (`AIBlueprintHelperLibrary.GetAIController` self)) (`self.AmmoName`) Current))

(fn `UserConstructionScript`
  (`parent.UserConstructionScript`)
  (`MeshComponent.SetVectorParameterValueOnMaterials` (`self.Mesh`) (`self.TintName`) (`KismetMathLibrary.Conv_LinearColorToVector` (`self.Color`))))