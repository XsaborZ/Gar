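; BP_BaseCharacter is a base character that equips a rifle and caches references to it and its animation Blueprint.
; On BeginPlay it sets the ChildActorComponent class from WeaponClass, then casts the spawned actor to BP_BaseRifle and the mesh's AnimInstance to ABP_CharacterAnimation.
; If either cast fails, it prints an error and destroys itself.
; Event bindings for rifle attack, reload and action end exist but are disconnected, so never run.
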(event `self.ReceiveBeginPlay`
  (`parent.ReceiveBeginPlay`)
  (`ChildActorComponent.SetChildActorClass` (`self.ChildActorComponent`) (`self.WeaponClass`))
  (`ChildActorComponent.SetChildActorClass` (`self.ChildActorComponent`) (`self.WeaponClass`))
  (bind _asbp_base_rifle (cast `/Game/Blueprints/Actors/BP_BaseRifle` (`ChildActorComponent.ChildActor` (`self.ChildActorComponent`)))
    (:`then`
      (set `self.WeaponObject` _asbp_base_rifle)
      (bind _asabp_character_animation (cast `/Game/Both/ABP_CharacterAnimation` (`SkeletalMeshComponent.GetAnimInstance` (`self.Mesh`)))
        (:`then`
          (set `self.AnimationBP` _asabp_character_animation))
        (:`CastFailed`
          (`KismetSystemLibrary.PrintString` "We need another animation BP")
          (`self.K2_DestroyActor`))))
    (:`CastFailed`
      (`KismetSystemLibrary.PrintString` "We need a Weapon")
      (`self.K2_DestroyActor`))))

(fn `UserConstructionScript`)