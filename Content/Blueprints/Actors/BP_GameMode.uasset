(fn `Add Enemu`)

(fn `Remove Enemy`
  (params (DestroyedActor :type "Actor Object Reference"))
  (bind _result (`/Engine/EditorBlueprintResources/StandardMacros.DecrementFloat` (`self.numberofenmemies`))
    (:`  `
      (if (not (> _result 0.0))
        (`KismetSystemLibrary.PrintString` "You Win" true true (struct :`R` 0.166948 :`G` 1.0 :`A` 1.0) 12.0)))))

(fn `UserConstructionScript`)