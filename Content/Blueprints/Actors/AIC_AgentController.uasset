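; AI controller for agents that runs a behavior tree and feeds it perceived targets through the Blackboard.
; On possess it starts the assigned behavior tree, and its construction script binds an event to the AI Perception target update.
; The perception handler writes a sensed actor to the player key and clears that key when sensing fails, with no filter on which actor triggered it.
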(event `self.ReceivePossess`
  (params (PossessedPawn :type "Pawn Object Reference"))
  (`self.RunBehaviorTree` (`self.BTAsset`)))

(fn `Handle Perception`
  (params (Actor :type "Actor Object Reference") (Stimulus :type "AIStimulus Structure"))
  (bind _player_name (`self.Player Name`))
  (bind _blackboard (`self.Blackboard`))
  (if (`.bSuccessfullySensed` (break `AIStimulus` Stimulus))
    (`BlackboardComponent.SetValueAsObject` _blackboard _player_name Actor)
    (else
      (`BlackboardComponent.ClearValue` _blackboard _player_name))))

(fn `UserConstructionScript`
  (add `AIPerceptionComponent.OnTargetPerceptionUpdated` (`self.AIPerception`) (`|CreateDelegate` :!event `Handle Perception`)))