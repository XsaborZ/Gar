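; BP_DamagePickup is a pickup actor that damages whoever picks it up.
; It overrides HandlePickup to run the parent pickup logic, then applies BaseDamage to the collecting actor with itself as the damage causer.
; The event graph and construction script add no behavior of their own, so all other pickup behavior is left to the parent class.
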(fn `HandlePickup`
  (params (Actor :type "Actor Object Reference") (`Hit Result` :type "HitResult Structure"))
  (`parent.HandlePickup` Actor `Hit Result`)
  (`GameplayStatics.ApplyDamage` Actor (`self.Base Damage`) null self))

(fn `UserConstructionScript`
  (`parent.UserConstructionScript`))